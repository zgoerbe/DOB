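; BP_FireBallPickup is a 2D pickup that grants fireballs to a BP_Character of one specific character type.
; When such a character overlaps its Box, it adds a random entry from the NoOfFireBalls array, clamped to that character's maximum.
; It then swaps the flipbook to SwitchPressed and destroys only the Box, so the used pickup stays visible but cannot trigger again.
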(event `self.Box.OnComponentBeginOverlap`
  (params (OverlappedComponent :type "PrimitiveComponent Object Reference") (OtherActor :type "Actor Object Reference") (OtherComp :type "PrimitiveComponent Object Reference") (OtherBodyIndex :type Integer) (bFromSweep :type Boolean) (SweepResult :type "HitResult Structure (by ref)"))
  (bind _asbp_character (cast `/Game/Blueprints/Character/BP_Character/BP_Character` OtherActor))
  (if (`|EnumEquality` (`/Game/Blueprints/Character/BP_Character/BP_Character.CharacterType` _asbp_character) "NewEnumerator3")
    (set `/Game/Blueprints/Character/BP_Character/BP_Character.NumberOfFireBalls` (`KismetMathLibrary.FClamp` (+ (`KismetArrayLibrary.Array_Random` (`self.NoOfFireBalls`)) (`/Game/Blueprints/Character/BP_Character/BP_Character.NumberOfFireBalls` _asbp_character)) 0.0 (`/Game/Blueprints/Character/BP_Character/BP_Character.MaxNumberOfFireBalls` _asbp_character)) _asbp_character)
    (`PaperFlipbookComponent.SetFlipbook` (`self.PaperFlipbook`) (`self.SwitchPressed`))
    (`ActorComponent.K2_DestroyComponent` (`self.Box`))))

(fn `UserConstructionScript`)