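; Player character for a 2D flipbook platformer, with abilities set by character type: Blue double-jumps and wall-jumps, Green sprints and dashes, Pink shoots limited fireballs.
; Flipbooks load from a data table at construction and reload every Tick, so type changes show during gameplay.
; Tick also picks the animation, line-traces for wall slides and turns the character through control yaw.
; Damage lowers health, shakes the camera and updates the HUD.
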(event `self.ReceiveBeginPlay`
  (bind _charactermovement (`self.CharacterMovement`))
  ;[1 0.7165 0.2045] Begin Play
  (set `CharacterMovementComponent.MaxWalkSpeed` (`self.PlayerWalkSpeed`) _charactermovement)
  (set `self.DefaultInAirControl` (`CharacterMovementComponent.AirControl` _charactermovement))
  (bind _returnvalue (`|CreateWidget` "/Game/Blueprints/HUD/WB_HUD.WB_HUD_C"))
  (bind _output_get (set `self.PlayerHUD` _returnvalue))
  (`UserWidget.AddToViewport` _output_get 0))

(event `UpdateAnimation`
  ;[0.4667 1 0.5271] Handle Animations
  (if (`self.IsDashing?`)
    (`PaperFlipbookComponent.SetFlipbook` (`self.Sprite`) (`self.Dashing`))
    (elif (`NavMovementComponent.IsFalling` (`self.CharacterMovement`))
      (if (`self.IsWallSliding?`)
        (`PaperFlipbookComponent.SetFlipbook` (`self.Sprite`) (`self.WallSliding`))
        (else
          (`PaperFlipbookComponent.SetFlipbook` (`self.Sprite`) (`self.CharacterJump`))))
      (else
        (`PaperFlipbookComponent.SetFlipbook` (`self.Sprite`) (select `bool` (> (`KismetMathLibrary.VSize` (`self.GetVelocity`)) 0.0) :`false` (`self.Front`) :`true` (`self.Walk`)))))))

(event `self.ReceiveTick`
  (params (DeltaSeconds :type "Float (single-precision)"))
  ;[0.5561 0.3524 1] Tick
  (`self.SetAnimationsDuringGameplay`)
  (`self.UpdateAnimation`)
  (`self.WallSlide`)
  (if (not (`self.IsWallSliding?`))
    (`self.CheckCharacterDirection` 0.0 180.0)))

(event `SetAnimationsDuringGameplay`
  ;[0.4667 1 0.5271] Handle Animations
  ;;[0.5771 1 0.593] Change Character Animations and Flipbooks during Gameplay
  (if (`|EnumEquality` (`self.CharacterType`) "NewEnumerator1")
    (`self.SetAnimations` "BlueCharacter")
    (set `self.CharacterTypeContainer` "NewEnumerator1")
    (elif (`|EnumEquality` (`self.CharacterType`) "NewEnumerator2")
      (`self.SetAnimations` "GreenCharacter")
      (set `self.CharacterTypeContainer` "NewEnumerator2")
      (elif (`|EnumEquality` (`self.CharacterType`) "NewEnumerator3")
        (`self.SetAnimations` "PinkCharacter")
        (set `self.CharacterTypeContainer` "NewEnumerator3")
        (else
          (set `self.CharacterTypeContainer` "NewEnumerator0"))))))

(event `InputAction|Jump`
  (params (Key :type "Key Structure"))
  (bind _returnvalue_x (`KismetMathLibrary.BreakVector` (`self.GetActorForwardVector`)))
  ;[0.4748 0.7244 1] Handle Input Events
  ;;[1 1 1] All Characters
  (:`Pressed`
    (if (`self.IsWallSliding?`)
      (`self.LaunchCharacter` (`KismetMathLibrary.MakeVector` (* _returnvalue_x -1500.0) 0.0 650.0) true true)
      (set `CharacterMovementComponent.AirControl` (`self.InAirControl`) (`self.CharacterMovement`))
      (else
        (set `CharacterMovementComponent.AirControl` (`self.DefaultInAirControl`) (`self.CharacterMovement`))
        (if (`|EnumEquality` (`self.CharacterType`) "NewEnumerator1")
          (set `self.JumpMaxCount` 2)
          (`self.Jump`)
          (else
            (set `self.JumpMaxCount` 1)
            (`self.Jump`))))))
  (:`Released`
    (`self.StopJumping`)))

(event `InputAxis|MoveRight`
  (params (AxisValue :type "Float (single-precision)"))
  ;[0.4748 0.7244 1] Handle Input Events
  ;;[1 1 1] All Characters
  (if (> AxisValue 0.0)
    (set `self.IsMovingRight?` true)
    (elif (< AxisValue 0.0)
      (set `self.IsMovingRight?` false)))
  (`self.AddMovementInput` (1.0 0.0 0.0) AxisValue))

(event `InputAction|Sprint`
  (params (Key :type "Key Structure"))
  (bind _returnvalue (`|EnumEquality` (`self.CharacterType`) "NewEnumerator2"))
  ;[0.4748 0.7244 1] Handle Input Events
  ;;[0 1 0.3378] Green Character
  (:`Pressed`
    (if _returnvalue
      (set `CharacterMovementComponent.MaxWalkSpeed` (`self.SprintSpeed`) (`self.CharacterMovement`))))
  (:`Released`
    (if _returnvalue
      (set `CharacterMovementComponent.MaxWalkSpeed` (`self.PlayerWalkSpeed`) (`self.CharacterMovement`)))))

(event `InputAction|Dash`
  (params (Key :type "Key Structure"))
  ;[0.4748 0.7244 1] Handle Input Events
  ;;[0 1 0.3378] Green Character
  (:`Pressed`
    (if (`|EnumEquality` (`self.CharacterType`) "NewEnumerator2")
      (`self.LaunchCharacter` (`KismetMathLibrary.MakeVector` (select `bool` (`self.IsMovingRight?`) :`false` -5000.0 :`true` 5000.0)) true)
      (set `self.IsDashing?` true)
      (set `CharacterMovementComponent.AirControl` (`self.InAirControl`) (`self.CharacterMovement`))
      (`KismetSystemLibrary.RetriggerableDelay` (`PaperFlipbook.GetTotalDuration` (`self.Dashing`)))
      (set `self.IsDashing?` false)
      (set `CharacterMovementComponent.AirControl` (`self.DefaultInAirControl`) (`self.CharacterMovement`)))))

(event `WallSlide`
  (bind _returnvalue (`self.K2_GetActorLocation`))
  ;[0.2604 0.3418 1] Wall Slide Implementation / Blue Character
  (if (`|EnumEquality` (`self.CharacterType`) "NewEnumerator1")
    (if (`NavMovementComponent.IsFalling` (`self.CharacterMovement`))
      (bind _outhit (`KismetSystemLibrary.LineTraceSingle` _returnvalue (+ (* (`self.GetActorForwardVector`) (55.0 0.0 0.0)) _returnvalue) "TraceTypeQuery1"))
      (set `self.IsWallSliding?` (`GameplayStatics.BreakHitResult` _outhit)))
    (else
      (set `self.IsWallSliding?` false))))

(event `InputAction|FireBallAttack`
  (params (Key :type "Key Structure"))
  ;[0.9433 0.5531 1] FireBallAttack / Pink Character
  (:`Pressed`
    (if (`|EnumEquality` (`self.CharacterType`) "NewEnumerator3")
      (if (> (`self.NumberOfFireBalls`) 0.0)
        (bind _returnvalue (`|SpawnActorFromClass` "/Game/Blueprints/Character/BP_Character/BP_FireBall.BP_FireBall_C" (`KismetMathLibrary.MakeTransform` (`SceneComponent.K2_GetComponentLocation` (`self.FireBallSpawn`)) (select `bool` (`self.IsMovingRight?`) :`false` (struct :`Yaw` -180.0) :!type "Rotator Structure")) "Undefined" "OverrideRootScale" self null))
        (`/Engine/EditorBlueprintResources/StandardMacros.IsValid` _returnvalue
          (:`Is Valid`
            (if (not (`/Game/Blueprints/Character/BP_Character/BP_FireBall.IsFireBallDestroyed?` _returnvalue))
              (`self.SetLifeSpan` _returnvalue 1.0)
              (bind _result (`/Engine/EditorBlueprintResources/StandardMacros.DecrementFloat` (`self.NumberOfFireBalls`))
                (:`  `
                  (set `self.NumberOfFireBalls` _result))))))))))

(event `Key|One`
  (params (Key :type "Key Structure")))

(event `self.ReceiveAnyDamage`
  (params (Damage :type "Float (single-precision)") (DamageType :type "DamageType Object Reference") (InstigatedBy :type "Controller Object Reference") (DamageCauser :type "Actor Object Reference"))
  ;[1 0.6127 0.4682] Recieve Damage and Add Camera Shake effect
  (set `self.Health` (- (`self.Health`) Damage))
  (`GameplayStatics.PlayWorldCameraShake` "/Game/Blueprints/Character/Camera/CameraShake.CameraShake_C" (`self.K2_GetActorLocation`) 0.0 500.0 1.0 true)
  (for _ (range 1 (+ (`KismetMathLibrary.FTrunc` Damage) 1))
    (`/Game/Blueprints/HUD/WB_HUD.UpdateHealth` (`self.PlayerHUD`))))

(fn `CheckCharacterDirection`
  (params (DirectionR :type "Float (double-precision)") (DirectionL :type "Float (double-precision)"))
  (bind _returnvalue (`self.GetController`))
  (bind _returnvalue_2 (`self.GetController`))
  (bind _velocity_x (`KismetMathLibrary.BreakVector` (`MovementComponent.Velocity` (`self.CharacterMovement`))))
  (`/Engine/EditorBlueprintResources/StandardMacros.CompareFloat` _velocity_x
    (:`>`
      (`/Engine/EditorBlueprintResources/StandardMacros.IsValid` _returnvalue_2 :!label _label
        (:`Is Valid`
          (`self.SetSpriteRotation` DirectionR _returnvalue_2))))
    (:`==`
      (if (`self.IsMovingRight?`)
        (goto _label)
        (else
          (`/Engine/EditorBlueprintResources/StandardMacros.IsValid` _returnvalue :!label _label_2
            (:`Is Valid`
              (`self.SetSpriteRotation` DirectionL _returnvalue))))))
    (:`<`
      (goto _label_2))))

(fn `SetAnimations`
  (params (Name :type Name))
  (locals (NewLocalVar_0 :type Name))
  (bind _outrownames (`DataTableFunctionLibrary.GetDataTableRowNames` "/Game/Blueprints/Character/DataTable/CharacterDataTable.CharacterDataTable"))
  (bind _returnvalue (`|GetDataTableRow` "/Game/Blueprints/Character/DataTable/CharacterDataTable.CharacterDataTable" (`|GetArrayItem` _outrownames (`KismetArrayLibrary.Array_Find` _outrownames Name)))
    (:`then`
      (if (`|EnumEquality` (break `/Game/Blueprints/Character/Structure/CharacterStructure` _returnvalue) (`self.CharacterType`))
        (set `self.Climb` (`.Climb_20_B947471E4E754E4017EAAAB8592064B3` (break `/Game/Blueprints/Character/Structure/CharacterStructure` _returnvalue)))
        (set `self.Duck` (`.Duck_21_76D1A13D4786227E340F5AAB519D9F77` (break `/Game/Blueprints/Character/Structure/CharacterStructure` _returnvalue)))
        (set `self.Front` (`.Front_22_C82110E24393D651EA0DD5B38A8260BB` (break `/Game/Blueprints/Character/Structure/CharacterStructure` _returnvalue)))
        (set `self.Hit` (`.Hit_23_F2B85A27468F07305EFFACB19F3561CF` (break `/Game/Blueprints/Character/Structure/CharacterStructure` _returnvalue)))
        (set `self.CharacterJump` (`.Jump_24_40B1A6704BF9C1A6462EE285D6CCC7CF` (break `/Game/Blueprints/Character/Structure/CharacterStructure` _returnvalue)))
        (set `self.Stand` (`.Stand_25_483A9E4F427AF18D4C939FBB5BFBC18D` (break `/Game/Blueprints/Character/Structure/CharacterStructure` _returnvalue)))
        (set `self.Swim` (`.Swim_26_A9C9C62C4CFFA1F51CBA28B31D77C7B7` (break `/Game/Blueprints/Character/Structure/CharacterStructure` _returnvalue)))
        (set `self.Walk` (`.Walk_27_B4595533482FF14E72EDEE801979F089` (break `/Game/Blueprints/Character/Structure/CharacterStructure` _returnvalue)))
        (set `self.Dashing` (`.Dashing_30_28D1CE61484361E503447DA914ABFA7A` (break `/Game/Blueprints/Character/Structure/CharacterStructure` _returnvalue)))
        (set `self.WallSliding` (`.WallSlide_33_2784148F44065EBB3955AE87EA74F744` (break `/Game/Blueprints/Character/Structure/CharacterStructure` _returnvalue)))))))

(fn `SetSpriteRotation`
  (params (RoationZ :type "Float (double-precision)") (Controller :type "Controller Object Reference"))
  (`Controller.SetControlRotation` Controller (`KismetMathLibrary.MakeRotator` 0.0 0.0 RoationZ)))

(fn `UserConstructionScript`
  ;[0.8846 0.6357 1] Construct the Character before the Game starts
  (bind _outrownames (`DataTableFunctionLibrary.GetDataTableRowNames` "/Game/Blueprints/Character/DataTable/CharacterDataTable.CharacterDataTable"))
  (for _array_element _outrownames
    (bind _returnvalue (`|GetDataTableRow` "/Game/Blueprints/Character/DataTable/CharacterDataTable.CharacterDataTable" _array_element)
      (:`then`
        (if (`|EnumEquality` (`self.CharacterType`) (break `/Game/Blueprints/Character/Structure/CharacterStructure` _returnvalue))
          (set `self.Climb` (`.Climb_20_B947471E4E754E4017EAAAB8592064B3` (break `/Game/Blueprints/Character/Structure/CharacterStructure` _returnvalue)))
          (set `self.Duck` (`.Duck_21_76D1A13D4786227E340F5AAB519D9F77` (break `/Game/Blueprints/Character/Structure/CharacterStructure` _returnvalue)))
          (set `self.Front` (`.Front_22_C82110E24393D651EA0DD5B38A8260BB` (break `/Game/Blueprints/Character/Structure/CharacterStructure` _returnvalue)))
          (set `self.Hit` (`.Hit_23_F2B85A27468F07305EFFACB19F3561CF` (break `/Game/Blueprints/Character/Structure/CharacterStructure` _returnvalue)))
          (set `self.CharacterJump` (`.Jump_24_40B1A6704BF9C1A6462EE285D6CCC7CF` (break `/Game/Blueprints/Character/Structure/CharacterStructure` _returnvalue)))
          (set `self.Stand` (`.Stand_25_483A9E4F427AF18D4C939FBB5BFBC18D` (break `/Game/Blueprints/Character/Structure/CharacterStructure` _returnvalue)))
          (set `self.Swim` (`.Swim_26_A9C9C62C4CFFA1F51CBA28B31D77C7B7` (break `/Game/Blueprints/Character/Structure/CharacterStructure` _returnvalue)))
          (set `self.Walk` (`.Walk_27_B4595533482FF14E72EDEE801979F089` (break `/Game/Blueprints/Character/Structure/CharacterStructure` _returnvalue)))
          (set `self.Dashing` (`.Dashing_30_28D1CE61484361E503447DA914ABFA7A` (break `/Game/Blueprints/Character/Structure/CharacterStructure` _returnvalue)))
          (set `self.WallSliding` (`.WallSlide_33_2784148F44065EBB3955AE87EA74F744` (break `/Game/Blueprints/Character/Structure/CharacterStructure` _returnvalue)))
          (`PaperFlipbookComponent.SetFlipbook` (`self.Sprite`) (`self.Front`))
          (set `self.HeartContainers` (`KismetMathLibrary.FTrunc` (`self.Health`))))))))