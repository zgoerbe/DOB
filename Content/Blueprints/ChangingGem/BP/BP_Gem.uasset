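; BP_Gem is a pickup that changes the player character's type when touched.
; On box overlap with a BP_Character, it sets CharacterType from its GemType enum through a branch chain, then destroys itself.
; The construction script scans GemDataTable for the row matching GemType and applies that row's GemColor sprite to its PaperSprite, so the look follows the chosen type in the editor.
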(event `self.Box.OnComponentBeginOverlap`
  (params (OverlappedComponent :type "PrimitiveComponent Object Reference") (OtherActor :type "Actor Object Reference") (OtherComp :type "PrimitiveComponent Object Reference") (OtherBodyIndex :type Integer) (bFromSweep :type Boolean) (SweepResult :type "HitResult Structure (by ref)"))
  ;[0.3637 0.8286 1] Change the Character Type when Character is Overlaping with the Gem and Destroy the Gem
  (bind _asbp_character (cast `/Game/Blueprints/Character/BP_Character/BP_Character` OtherActor))
  (if (`|EnumEquality` (`self.GemType`) "NewEnumerator0")
    (set `/Game/Blueprints/Character/BP_Character/BP_Character.CharacterType` "NewEnumerator2" _asbp_character)
    (`self.K2_DestroyActor` :!label _label)
    (elif (`|EnumEquality` (`self.GemType`) "NewEnumerator1")
      (set `/Game/Blueprints/Character/BP_Character/BP_Character.CharacterType` "NewEnumerator1" _asbp_character)
      (goto _label)
      (elif (`|EnumEquality` (`self.GemType`) "NewEnumerator2")
        (set `/Game/Blueprints/Character/BP_Character/BP_Character.CharacterType` "NewEnumerator3" _asbp_character)
        (goto _label)))))

(fn `UserConstructionScript`
  (bind _outrownames (`DataTableFunctionLibrary.GetDataTableRowNames` "/Game/Blueprints/ChangingGem/DataTable/GemDataTable.GemDataTable"))
  (for _array_element _outrownames
    (bind _returnvalue (`|GetDataTableRow` "/Game/Blueprints/ChangingGem/DataTable/GemDataTable.GemDataTable" _array_element)
      (:`then`
        (if (`|EnumEquality` (`self.GemType`) (break `/Game/Blueprints/ChangingGem/Structure/GemStructure` _returnvalue))
          (bind _output_get (set `self.GemColor` (`.GemColor_2_9CB0BD994C074D353B03D9A0BF1DA858` (break `/Game/Blueprints/ChangingGem/Structure/GemStructure` _returnvalue))))
          (`PaperSpriteComponent.SetSprite` (`self.PaperSprite`) _output_get))))))