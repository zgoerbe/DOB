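; BP_Spring is a spring pad that launches BP_Character upward when it overlaps the Box trigger.
; The launch uses the SpringLaunchVelocity variable and overrides both horizontal and vertical velocity.
; The flipbook then swaps to the active spring animation and returns to the inactive one after a delay equal to that animation's duration.
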(event `self.Box.OnComponentBeginOverlap`
  (params (OverlappedComponent :type "PrimitiveComponent Object Reference") (OtherActor :type "Actor Object Reference") (OtherComp :type "PrimitiveComponent Object Reference") (OtherBodyIndex :type Integer) (bFromSweep :type Boolean) (SweepResult :type "HitResult Structure (by ref)"))
  (bind _activespring (`self.ActiveSpring`))
  (bind _asbp_character (cast `/Game/Blueprints/Character/BP_Character/BP_Character` OtherActor))
  (`Character.LaunchCharacter` _asbp_character (`KismetMathLibrary.MakeVector` 0.0 0.0 (`self.SpringLaunchVelocity`)) true true)
  (`PaperFlipbookComponent.SetFlipbook` (`self.spring_FlipbookInactive`) _activespring)
  (`KismetSystemLibrary.Delay` (`PaperFlipbook.GetTotalDuration` _activespring))
  (`PaperFlipbookComponent.SetFlipbook` (`self.spring_FlipbookInactive`) (`self.InactiveSpring`)))

(fn `UserConstructionScript`)