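; BP_Lock is a level goal: a lock the player character opens with a key, revealing a switch that wins the level.
; Overlapping the lock box with BP_Character holding a key plays the unlock sound, shows the switch and destroys the lock and its trigger.
; Overlapping the win box swaps the switch sprite, plays a sound, then opens the WinMenu level after the sound's duration plus a short delay.
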(event `self.LockBox.OnComponentBeginOverlap`
  (params (OverlappedComponent :type "PrimitiveComponent Object Reference") (OtherActor :type "Actor Object Reference") (OtherComp :type "PrimitiveComponent Object Reference") (OtherBodyIndex :type Integer) (bFromSweep :type Boolean) (SweepResult :type "HitResult Structure (by ref)"))
  (bind _asbp_character (cast `/Game/Blueprints/Character/BP_Character/BP_Character` OtherActor))
  (if (`/Game/Blueprints/Character/BP_Character/BP_Character.HasKey?` _asbp_character)
    (`GameplayStatics.PlaySound2D` (`self.UnlockSound`) 1.0 1.0 0.0 null null)
    (`SceneComponent.SetVisibility` (`self.WinSwitch`) true false)
    (`ActorComponent.K2_DestroyComponent` (`self.Lock`))
    (`ActorComponent.K2_DestroyComponent` (`self.LockBox`))))

(event `self.WinBox.OnComponentBeginOverlap`
  (params (OverlappedComponent :type "PrimitiveComponent Object Reference") (OtherActor :type "Actor Object Reference") (OtherComp :type "PrimitiveComponent Object Reference") (OtherBodyIndex :type Integer) (bFromSweep :type Boolean) (SweepResult :type "HitResult Structure (by ref)"))
  (bind _activateswitchsound (`self.ActivateSwitchSound`))
  (cast `/Game/Blueprints/Character/BP_Character/BP_Character` OtherActor)
  (`PaperSpriteComponent.SetSprite` (`self.WinSwitch`) (`self.ActivatedSwitch`))
  (`GameplayStatics.PlaySound2D` _activateswitchsound 1.0 1.0 0.0 null null)
  (`KismetSystemLibrary.Delay` (+ (`SoundBase.Duration` _activateswitchsound) 3.0))
  (`GameplayStatics.OpenLevel` "WinMenu"))

(fn `UserConstructionScript`)