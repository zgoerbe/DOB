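; Side-scrolling flipbook enemy that patrols or stands still, attacks the player and can be stomped or damaged.
; The construction script loads flipbooks and health from a data table by EnemyType.
; Tick selects animations from state flags, handles death cleanup, and uses line traces to pause and reverse at walls or ledges.
; An overlap box runs a looping timer for cooldown-gated, trace-checked attacks, while another detects falling-player stomps and bounces the player.
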(event `self.ReceiveBeginPlay`
  ;[0.4225 1 0.8899] Set up Enemy Flipbooks and Random Enemy Movement Direction
  (if (`|EnumEquality` (`self.EnemyType`) "NewEnumerator5")
    (set `self.CanMove?` false)
    (else
      (set `self.CanMove?` (`KismetArrayLibrary.Array_Random` (`self.MoveOrStayArray`)))
      (set `self.MovementDirection` (`KismetArrayLibrary.Array_Random` (`self.MoveDirectionValues`))))))

(event `self.ReceiveTick`
  (params (DeltaSeconds :type "Float (single-precision)"))
  ;[0.7691 0.4386 1] Tick
  (`self.HandleAnimation`)
  (`self.HandleMovement`))

(event `HandleAnimation`
  (bind _deadbody (`self.DeadBody`))
  ;[0.1368 1 0.4702] Handle Animations
  (if (`self.IsEnemyDead?`)
    (`PaperFlipbookComponent.SetFlipbook` (`self.Sprite`) _deadbody)
    (`PrimitiveComponent.SetCollisionResponseToChannel` (`self.CapsuleComponent`) "ECC_Pawn" "ECR_Ignore")
    (`PrimitiveComponent.SetCollisionEnabled` (`self.Box`) "NoCollision")
    (`KismetSystemLibrary.Delay` (+ (`PaperFlipbook.GetTotalDuration` _deadbody) 3.0))
    (`self.K2_DestroyActor`)
    (elif (`self.EnemyDamaged?`)
      (`PaperFlipbookComponent.SetFlipbook` (`self.Sprite`) (`self.Hit`))
      (elif (`self.IsAttacking?`)
        (`PaperFlipbookComponent.SetFlipbook` (`self.Sprite`) (`self.Attack`))
        (else
          (`PaperFlipbookComponent.SetFlipbook` (`self.Sprite`) (select `bool` (> (`KismetMathLibrary.VSize` (`MovementComponent.Velocity` (`self.CharacterMovement`))) 0.0) :`false` (`self.Idle`) :`true` (`self.Move`))))))))

(event `HandleMovement`
  (bind _returnvalue (`self.K2_GetActorLocation`))
  (bind _returnvalue_2 (`self.K2_GetActorLocation`))
  ;[1 0.6117 0.8417] Handle Movement
  (`|ExecutionSequence`
    (:`then_0`
      (if (> (`self.MovementDirection`) 0.0)
        (`self.K2_SetActorRotation` (struct :`Yaw` 180.0))
        (else
          (`self.K2_SetActorRotation` (struct)))))
    (:`then_1`
      (if (`self.CanMove?`)
        (if (not (or (`self.IsEnemyDead?`) (`self.EnemyDamaged?`) (`self.IsAttacking?`)))
          (`self.AddMovementInput` (1.0 0.0 0.0) (`self.MovementDirection`))
          (`|ExecutionSequence`
            (:`then_0`
              ;;[1 0.9942 0.7118] Check for Wall
              (bind (_outhit _returnvalue_3) (`KismetSystemLibrary.LineTraceSingle` _returnvalue_2 (+ _returnvalue_2 (* (`self.GetActorForwardVector`) (`KismetMathLibrary.MakeVector` (* (`self.LineTraceLength`) -1.0)))) "TraceTypeQuery1"))
              (if _returnvalue_3
                (`/Engine/EditorBlueprintResources/StandardMacros.DoOnce` false :!label _label
                  (:`Completed`
                    (set `CharacterMovementComponent.MaxWalkSpeed` 0.0 (`self.CharacterMovement`))
                    (`KismetSystemLibrary.Delay` (`self.EnemyWaitTime`))
                    (set `CharacterMovementComponent.MaxWalkSpeed` (`self.EnemyWalkSpeed`) (`self.CharacterMovement`))
                    (set `self.MovementDirection` (* (`self.MovementDirection`) -1.0))
                    (goto _label :!via `Reset`)))))
            (:`then_1`
              ;;[0.5354 0.6305 1] Check if on edge
              (bind (_outhit_2 _returnvalue_4) (`KismetSystemLibrary.LineTraceSingle` _returnvalue (+ (- _returnvalue (0.0 0.0 100.0)) (* (`self.GetActorForwardVector`) (`KismetMathLibrary.MakeVector` (* (`self.LineTraceLength`) -1.0)))) "TraceTypeQuery1"))
              (if (not _returnvalue_4)
                (goto _label)))))))))

(event `ApplyJumpDamage`
  ;[1 0.599 0.3149] Recieve Damage
  (if (<= (`self.EnemyHealth`) 0.0) :!label _label_2
    (set `self.IsEnemyDead?` true)
    (else
      (set `self.EnemyDamaged?` true)
      (`KismetSystemLibrary.RetriggerableDelay` (`PaperFlipbook.GetTotalDuration` (`self.Hit`)))
      (set `self.EnemyDamaged?` false))))

(event `self.ReceiveAnyDamage`
  (params (Damage :type "Float (single-precision)") (DamageType :type "DamageType Object Reference") (InstigatedBy :type "Controller Object Reference") (DamageCauser :type "Actor Object Reference"))
  (bind _returnvalue_x (`KismetMathLibrary.BreakVector` (`KismetMathLibrary.Normal` (`KismetMathLibrary.GetDirectionUnitVector` (`self.K2_GetActorLocation` DamageCauser) (`self.K2_GetActorLocation`)))))
  ;[1 0.599 0.3149] Recieve Damage
  (set `self.EnemyHealth` (- (`self.EnemyHealth`) Damage))
  (`self.LaunchCharacter` (`KismetMathLibrary.MakeVector` (* (select `bool` (< _returnvalue_x 0.0) :`false` -1.0 :`true` 1.0) -1500.0)) true true)
  (goto _label_2))

(event `self.Box.OnComponentBeginOverlap`
  (params (OverlappedComponent :type "PrimitiveComponent Object Reference") (OtherActor :type "Actor Object Reference") (OtherComp :type "PrimitiveComponent Object Reference") (OtherBodyIndex :type Integer) (bFromSweep :type Boolean) (SweepResult :type "HitResult Structure (by ref)"))
  ;[0.4533 1 0.2343] Apply Jump Damage
  (bind _asbp_character (cast `/Game/Blueprints/Character/BP_Character/BP_Character` OtherActor))
  (if (`NavMovementComponent.IsFalling` (`Character.CharacterMovement` _asbp_character))
    (set `self.EnemyHealth` (- (`self.EnemyHealth`) (`/Game/Blueprints/Character/BP_Character/BP_Character.JumpDamage` _asbp_character)))
    (`self.ApplyJumpDamage`)
    (`self.LaunchCharacter` _asbp_character (0.0 0.0 500.0) true true)))

(event `AttackPlayer`
  (bind _returnvalue (`self.K2_GetActorLocation`))
  ;[1 0.6502 0.3429] Apply Damage to Player
  (if (not (`self.IsEnemyDead?`))
    (`/Engine/EditorBlueprintResources/StandardMacros.DoOnce` false :!label _label_3
      (:`Completed`
        (set `self.IsAttacking?` true)
        (`KismetSystemLibrary.Delay` (`PaperFlipbook.GetTotalDuration` (`self.Attack`)))
        (`|ExecutionSequence`
          (:`then_0`
            (set `self.IsAttacking?` false))
          (:`then_1`
            (bind _outhit (`KismetSystemLibrary.LineTraceSingleForObjects` _returnvalue (+ (* (`self.GetActorForwardVector`) (`KismetMathLibrary.MakeVector` (* (`self.LineTraceLength`) -1.0))) _returnvalue) (`|MakeArray` "ObjectTypeQuery3" :!type "EObjectTypeQuery Enum") false (`|MakeArray` self :!type "Actor Object Reference") "ForDuration"))
            (bind (_bblockinghit _binitialoverlap _time _distance _location _impactpoint _normal _impactnormal _physmat _hitactor) (`GameplayStatics.BreakHitResult` _outhit))
            (if (== (`GameplayStatics.GetPlayerCharacter` 0) _hitactor)
              (`GameplayStatics.ApplyDamage` _hitactor (`self.EnemyDamage`)))
            (`KismetSystemLibrary.Delay` (`self.CoolDown`))
            (goto _label_3 :!via `Reset`)))))))

(event `self.AttackBox.OnComponentBeginOverlap`
  (params (OverlappedComponent :type "PrimitiveComponent Object Reference") (OtherActor :type "Actor Object Reference") (OtherComp :type "PrimitiveComponent Object Reference") (OtherBodyIndex :type Integer) (bFromSweep :type Boolean) (SweepResult :type "HitResult Structure (by ref)"))
  ;[1 0.6502 0.3429] Apply Damage to Player
  (cast `/Game/Blueprints/Character/BP_Character/BP_Character` OtherActor)
  (bind _returnvalue (`KismetSystemLibrary.K2_SetTimerDelegate` (delegate `AttackPlayer`) 0.1 true))
  (set `self.AttackEvent` _returnvalue))

(event `self.AttackBox.OnComponentEndOverlap`
  (params (OverlappedComponent :type "PrimitiveComponent Object Reference") (OtherActor :type "Actor Object Reference") (OtherComp :type "PrimitiveComponent Object Reference") (OtherBodyIndex :type Integer))
  ;[1 0.6502 0.3429] Apply Damage to Player
  (cast `/Game/Blueprints/Character/BP_Character/BP_Character` OtherActor)
  (`KismetSystemLibrary.K2_ClearAndInvalidateTimerHandle` (`self.AttackEvent`))
  (goto _label_3 :!via `Reset`))

(fn `UserConstructionScript`
  ;[0.3908 0.6828 1] Construct the Enemies before the Game Starts
  (bind _outrownames (`DataTableFunctionLibrary.GetDataTableRowNames` "/Game/Blueprints/Enemy/DataTable/EnemyDataTable.EnemyDataTable"))
  (for _array_element _outrownames
    (bind _returnvalue (`|GetDataTableRow` "/Game/Blueprints/Enemy/DataTable/EnemyDataTable.EnemyDataTable" _array_element)
      (:`then`
        (if (`|EnumEquality` (break `/Game/Blueprints/Enemy/Structure/EnemyStructure` _returnvalue) (`self.EnemyType`))
          (set `self.Idle` (`.Idle_14_B7D3C605411CAACE454788A33C3EC339` (break `/Game/Blueprints/Enemy/Structure/EnemyStructure` _returnvalue)))
          (set `self.Move` (`.Move_10_5FA651204B62C11B40D40EBF96038A58` (break `/Game/Blueprints/Enemy/Structure/EnemyStructure` _returnvalue)))
          (set `self.Attack` (`.Attack_20_E7D7ADF84AA6E5769F7C5CBD55F0ECCB` (break `/Game/Blueprints/Enemy/Structure/EnemyStructure` _returnvalue)))
          (set `self.Hit` (`.Hit_11_BF2A68874434BC0D71EBA7A689F016DE` (break `/Game/Blueprints/Enemy/Structure/EnemyStructure` _returnvalue)))
          (set `self.DeadBody` (`.DeadBody_12_AF60D88B4E79B4200755AF8B2D56B10C` (break `/Game/Blueprints/Enemy/Structure/EnemyStructure` _returnvalue)))
          (set `self.EnemyHealth` (`.EnemyHealth_17_56C1EA1B41CC2D261CE169B574C0DFE6` (break `/Game/Blueprints/Enemy/Structure/EnemyStructure` _returnvalue)))
          (`PaperFlipbookComponent.SetFlipbook` (`self.Sprite`) (`self.Idle`)))))))